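; BP_FloorButton is a floor switch that reports door switch activation and deactivation through the game state.
; Its Sphere's begin and end overlaps publish the corresponding messages to the game state, without filtering the overlapping actor.
; It subscribes to BP_GameState's door-state change event and toggles IsActive when the broadcast ID matches its SwitchID.
; Getter functions expose both the ID and the active state.
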(event OnComponentBeginOverlap(Sphere)
  (params (OverlappedComponent :type Primitive%20Component%20Object%20Reference) (OtherActor :type Actor%20Object%20Reference) (OtherComp :type Primitive%20Component%20Object%20Reference) (OtherBodyIndex :type Integer) (bFromSweep :type Boolean) (SweepResult :type Hit%20Result%20Structure%20%28by%20ref%29))
  (Class|BPIDoorEventsManager|PublishDoorSwitchActivatedEvent(Message) (Game|GetGameState)))

(event OnComponentEndOverlap(Sphere)
  (params (OverlappedComponent :type Primitive%20Component%20Object%20Reference) (OtherActor :type Actor%20Object%20Reference) (OtherComp :type Primitive%20Component%20Object%20Reference) (OtherBodyIndex :type Integer))
  (Class|BPIDoorEventsManager|PublishDoorSwitchDeactivatedEvent(Message) (Game|GetGameState)))

(event Custom|SwitchDoorStateChanged
  (params (ButtonID :type EButtonsIDs%20Enum :default "NewEnumerator0"))
  (if (Utilities|Enum|Equal(Enum) ButtonID (Variables|Default|GetSwitchID))
    (Variables|Default|SetbIsActive (not (Variables|Default|GetbIsActive)))))

(event EventBeginPlay
  (bind _asbp_game_state (Utilities|Casting|CastToBP_GameState (Game|GetGameState)))
  (EventDispatchers|BindEventtoOnSwitchDoorStateChange _asbp_game_state (delegate Custom|SwitchDoorStateChanged)))

(event Collision|EventActorBeginOverlap
  (params (OtherActor :type Actor%20Object%20Reference)))

(event EventTick
  (params (DeltaSeconds :type Float%20%28single-precision%29)))

(fn ConstructionScript)

(fn GetButtonID
  (return (Variables|Default|GetSwitchID)))

(fn GetIsActive
  (return (Variables|Default|GetbIsActive)))