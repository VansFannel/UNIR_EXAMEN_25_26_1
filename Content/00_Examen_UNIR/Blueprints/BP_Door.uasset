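; BP_Door is a two-leaf sliding door that opens and closes according to the state of its assigned buttons.
; It binds to the BP_GameState switch-change event and rechecks Buttons on each broadcast, though AreAllActivated keeps only the last button's state.
; A timeline plays or reverses, guarded by IsDoorClosed, setting each leaf's relative location to the actor location minus or plus the animated offset.
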(event Custom|OnSwitchDoorStateChange
  (params (ButtonID :type EButtonsIDs%20Enum :default "NewEnumerator0"))
  (CallFunction|CheckSwitchsDoorState))

(event Custom|OpenDoor_Event
  (if (Variables|Default|GetbIsDoorClosed)
    (Variables|Default|SetbIsDoorClosed false)
    (bind _dooranimation (Timeline|OpenCloseAnimation Play)
      (:Update
        (Transformation|SetRelativeLocation (Variables|Default|GetLeaf01) (- (Transformation|GetActorLocation) _dooranimation) false false)
        (Transformation|SetRelativeLocation (Variables|Default|GetLeaf02) (+ (Transformation|GetActorLocation) _dooranimation) false false)))))

(event Custom|CloseDoor_Event
  (if (not (Variables|Default|GetbIsDoorClosed))
    (Variables|Default|SetbIsDoorClosed true)
    (bind _dooranimation (Timeline|OpenCloseAnimation Reverse)
      (:Update
        (Transformation|SetRelativeLocation (Variables|Default|GetLeaf01) (- (Transformation|GetActorLocation) _dooranimation) false false)
        (Transformation|SetRelativeLocation (Variables|Default|GetLeaf02) (+ (Transformation|GetActorLocation) _dooranimation) false false)))))

(event EventBeginPlay
  (bind _asbp_game_state (Utilities|Casting|CastToBP_GameState (Game|GetGameState)))
  (EventDispatchers|BindEventtoOnSwitchDoorStateChange _asbp_game_state (delegate Custom|OnSwitchDoorStateChange)))

(fn ConstructionScript)

(fn CheckSwitchsDoorState
  (for _array_element (Variables|Default|GetButtons)
    (bind _isactive (Default|GetIsActive _array_element))
    (LocalVariables|SetbAreAllActivated _isactive))
  (if (LocalVariables|GetbAreAllActivated)
    (CallFunction|OpenDoorEvent)
    (else
      (CallFunction|CloseDoorEvent))))